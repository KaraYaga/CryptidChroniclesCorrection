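; BP_DakotaTomJr is a character Blueprint that handles taking damage and dying.
; AnyDamage subtracts from Health, clamped at zero, and prints the new value.
; At zero Health it adds a WBP_GameOver widget to the viewport, shows the mouse cursor, sets game-only input mode and destroys the actor.
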(event Game|Damage|EventAnyDamage
  (params (Damage :type Float%20%28single-precision%29) (DamageType :type Damage%20Type%20Object%20Reference) (InstigatedBy :type Controller%20Object%20Reference) (DamageCauser :type Actor%20Object%20Reference))
  (bind _returnvalue (Game|GetPlayerController 0))
  ;[1 1 1] Take Damage / DIe
  (bind _output_get (Variables|Default|SetHealth (Math|Float|Max(Float) (- (Variables|Default|GetHealth) Damage) 0.0)))
  (Development|PrintString (Utilities|String|ToString(Float) _output_get))
  (if (== (Variables|Default|GetHealth) 0.0)
    (bind _returnvalue_2 (UserInterface|CreateWidget "/Game/UI/WBP_GameOver.WBP_GameOver_C"))
    (UserInterface|Viewport|AddtoViewport _returnvalue_2 0)
    (Variables|/Script/Engine.PlayerController|SetbShowMouseCursor _returnvalue true)
    (Input|SetInputModeGameOnly _returnvalue false)
    (Actor|DestroyActor)))

(fn ConstructionScript
  (|CallParentFunction))
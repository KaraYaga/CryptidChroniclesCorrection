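; Yeti enemy that turns to face the Dakota Tom Jr character when pawn sensing sees it and attacks at range.
; While CanAttack is set, it spawns a projectile at SpawnProjectileLocation, then after a short delay stops that projectile's physics.
; Damage is applied directly to the seen character on that timer, independent of projectile collision.
; CanAttack clears only after that delay, then resets following a brief cooldown.
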(event OnSeePawn(PawnSensing)
  (params (Pawn :type Pawn%20Object%20Reference))
  (bind _asbp_dakota_tom_jr (Utilities|Casting|CastToBP_DakotaTomJr Pawn))
  (Transformation|SetActorRotation (Math|Rotator|FindLookatRotation (Transformation|GetActorLocation) (Transformation|GetActorLocation _asbp_dakota_tom_jr)))
  (if (Variables|Default|GetCanAttack)
    (bind _returnvalue (Game|SpawnActorfromClass "/Game/Characters/Yeti/BP_YetiProjectile.BP_YetiProjectile_C" (Transformation|GetWorldTransform (Variables|Default|GetSpawnProjectileLocation)) "Undefined" "MultiplyWithRoot" 0 0))
    (Utilities|FlowControl|Delay 0.2)
    (Physics|SetSimulatePhysics (Variables|/Game/Characters/Yeti/BP_YetiProjectile.BP_YetiProjectile_C|GetSphere _returnvalue) false)
    (Game|Damage|ApplyDamage _asbp_dakota_tom_jr 1e+01 0 0)
    (Variables|Default|SetCanAttack false)
    (Utilities|FlowControl|Delay 0.5)
    (Variables|Default|SetCanAttack true)))

(fn ConstructionScript
  (|CallParentFunction))
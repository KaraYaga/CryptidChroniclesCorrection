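; Base character Blueprint that sets its walk speed on BeginPlay and reacts to the physical surface beneath it.
; Every Tick, a debug-drawn downward line trace on Visibility reads the hit's physical material surface type.
; Ice zeroes ground friction and braking deceleration for sliding, while other surfaces restore fixed values.
; Fire is the exception, printing a pain message and leaving movement settings unchanged.
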(event EventBeginPlay
  (Variables|/Script/Engine.CharacterMovementComponent|SetMaxWalkSpeed (Variables|Character|GetCharacterMovement) (Variables|Default|GetWalkSpeed)))

(event EventTick
  (params (DeltaSeconds :type Float%20%28single-precision%29))
  (bind _returnvalue (Transformation|GetActorLocation))
  (bind (_outhit _returnvalue_2) (Collision|LineTraceByChannel _returnvalue (- _returnvalue "0.000000,0.000000,1000.000000") "TraceTypeQuery1" false 0 "ForDuration"))
  (if _returnvalue_2
    (switch Utilities|FlowControl|Switch|SwitchonEPhysicalSurface (Variables|/Script/PhysicsCore.PhysicalMaterial|GetSurfaceType (.PhysMat (Collision|BreakHitResult _outhit)))
      (:SurfaceType_Default
        (Variables|/Script/Engine.CharacterMovementComponent|SetBrakingDecelerationWalking (Variables|Character|GetCharacterMovement) 2048.0)
        (Variables|/Script/Engine.CharacterMovementComponent|SetGroundFriction (Variables|Character|GetCharacterMovement) 8.0))
      (:SurfaceType1
        (Variables|/Script/Engine.CharacterMovementComponent|SetBrakingDecelerationWalking (Variables|Character|GetCharacterMovement) 0.0)
        (Variables|/Script/Engine.CharacterMovementComponent|SetGroundFriction (Variables|Character|GetCharacterMovement) 0.0))
      (:SurfaceType2
        (Development|PrintString "Aoutch")))))

(fn ConstructionScript)
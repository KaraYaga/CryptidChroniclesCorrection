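; PC_Player is the player controller that turns Enhanced Input actions into pawn movement, camera look and pausing.
; It registers IMC_Player on BeginPlay, then moves the controlled pawn along forward and right vectors taken from the desired rotation.
; Camera input drives yaw and pitch, with InvertCamera flipping the pitch sign.
; The pause action adds W_PauseMenu to HUD_Player's menu slot and pauses the game.
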(event Input|EnhancedActionEvents|EnhancedInputActionIA_MoveCamera
  (params (ActionValue :type Vector%202D%20Structure) (ElapsedSeconds :type Float%20%28double-precision%29) (TriggeredSeconds :type Float%20%28double-precision%29) (InputAction :type Input%20Action%20Object%20Reference :default "/Game/_GameManager/Inputs/IA_MoveCamera.IA_MoveCamera"))
  (bind (_x _y) (Math|Vector2D|BreakVector2D ActionValue))
  (:Triggered
    (Class|PlayerController|AddYawInput _x)
    (Class|PlayerController|AddPitchInput (* _y (Math|Float|SelectFloat 1.0 -1.0 (Variables|Default|GetInvertCamera?))))))

(event Input|EnhancedActionEvents|EnhancedInputActionIA_Move
  (params (ActionValue :type Vector%202D%20Structure) (ElapsedSeconds :type Float%20%28double-precision%29) (TriggeredSeconds :type Float%20%28double-precision%29) (InputAction :type Input%20Action%20Object%20Reference :default "/Game/_GameManager/Inputs/IA_Move.IA_Move"))
  (bind (_x _y) (Math|Vector2D|BreakVector2D ActionValue))
  (:Triggered
    (Pawn|Input|AddMovementInput (Pawn|GetControlledPawn) (Math|Vector|GetForwardVector (Pawn|GetDesiredRotation)) _y false)
    (Pawn|Input|AddMovementInput (Pawn|GetControlledPawn) (Math|Vector|GetRightVector (Pawn|GetDesiredRotation)) _x false)))

(event Input|EnhancedActionEvents|EnhancedInputActionIA_Pause
  (params (ActionValue :type Boolean) (ElapsedSeconds :type Float%20%28double-precision%29) (TriggeredSeconds :type Float%20%28double-precision%29) (InputAction :type Input%20Action%20Object%20Reference :default "/Game/_GameManager/Inputs/IA_Pause.IA_Pause"))
  (:Triggered
    (bind _ashud_player (Utilities|Casting|CastToHUD_Player (HUD|GetHUD)))
    (Default|AddtoMenuSlot _ashud_player "/Game/UI/W_PauseMenu.W_PauseMenu_C")
    (Game|SetGamePaused true)))

(event EventBeginPlay
  (Input|AddMappingContext (PlayerController|LocalPlayerSubsystems|GetEnhancedInputLocalPlayerSubsystem) "/Game/_GameManager/Inputs/IMC_Player.IMC_Player" 0 "(bIgnoreAllPressedKeysUntilRelease=True,bForceImmediately=False)"))

(fn ConstructionScript)